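; Elevator platform for the side-scroller that makes a round trip when the player character enters its collision volume.
; Begin overlap starts a timeline that lerps the Elevator's relative location from A to B.
; After a fixed delay, counted from the start of that move, a second timeline lerps it back, both without sweeping.
; End overlap only casts to the character and triggers nothing.
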(event `self.Collision.OnComponentEndOverlap`
  (params (OverlappedComponent :type "PrimitiveComponent Object Reference") (OtherActor :type "Actor Object Reference") (OtherComp :type "PrimitiveComponent Object Reference") (OtherBodyIndex :type Integer))
  (cast `/Game/2DSideScrollerBP/Blueprints/2DSideScrollerCharacter` OtherActor))

(event `self.Collision.OnComponentBeginOverlap`
  (params (OverlappedComponent :type "PrimitiveComponent Object Reference") (OtherActor :type "Actor Object Reference") (OtherComp :type "PrimitiveComponent Object Reference") (OtherBodyIndex :type Integer) (bFromSweep :type Boolean) (SweepResult :type "HitResult Structure (by ref)"))
  (cast `/Game/2DSideScrollerBP/Blueprints/2DSideScrollerCharacter` OtherActor)
  (`self.PlatformBegin`)
  (`KismetSystemLibrary.Delay` 10.0)
  (`self.PlatformReverse`))

(event `PlatformBegin`
  (bind (_direction _newtrack_0) (`Timeline|Begin` :!via `PlayFromStart`)
    (:`Update`
      (`SceneComponent.K2_SetRelativeLocation` (`self.Elevator`) (`KismetMathLibrary.VLerp` (`self.A`) (`self.B`) _newtrack_0) false false))))

(event `PlatformReverse`
  (bind (_direction _newtrack_0) (`Timeline|Timeline_0` :!via `PlayFromStart`)
    (:`Update`
      (`SceneComponent.K2_SetRelativeLocation` (`self.Elevator`) (`KismetMathLibrary.VLerp` (`self.B`) (`self.A`) _newtrack_0) false false))))

(fn `UserConstructionScript`)